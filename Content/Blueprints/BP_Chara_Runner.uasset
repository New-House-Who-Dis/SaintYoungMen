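; Auto-running player character that moves along world +X at Speed every tick, with jumping through Enhanced Input.
; Its MessageText shows an opening line on BeginPlay, then a random entry from Messages on each jump, shrinking the text for long lines.
; Jumping also sends the Locomotion animation state machine to Airborne via JumpToNode.
; Camera-facing rotation and the jump back to Run are left disconnected.
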(event `EnhancedInput|/Game/Characters/Input/Actions/IA_Jump`
  (params (ActionValue :type Boolean) (ElapsedSeconds :type "Float (double-precision)") (TriggeredSeconds :type "Float (double-precision)") (InputAction :type "InputAction Object Reference" :default "/Game/Characters/Input/Actions/IA_Jump.IA_Jump"))
  (:`Triggered`
    (`self.Jump`)))

(event `self.ReceiveBeginPlay`
  (`TextRenderComponent.K2_SetText` (`self.MessageText`) (`|FormatText` "...Why is it so hot?"))
  (bind _asplayer_controller (cast `PlayerController` (`self.GetController`)))
  (bind _returnvalue (pcsubsystem `EnhancedInputLocalPlayerSubsystem` _asplayer_controller))
  (`/Engine/EditorBlueprintResources/StandardMacros.IsValid` _returnvalue
    (:`Is Valid`
      (`EnhancedInputSubsystemInterface.AddMappingContext` _returnvalue "/Game/Characters/Input/IMC_Default.IMC_Default" 0 (struct)))))

(event `self.ReceiveTick`
  (params (DeltaSeconds :type "Float (single-precision)"))
  (`self.AddMovementInput` (1.0 0.0 0.0) (`self.Speed`)))

(event `self.OnJumped`
  (bind _messagetext (`self.MessageText`))
  (bind _output_get (set `self.Message` (`KismetArrayLibrary.Array_Random` (`self.Messages`))))
  (`TextRenderComponent.K2_SetText` _messagetext _output_get)
  (if (>= (`KismetStringLibrary.Len` (`KismetTextLibrary.Conv_TextToString` _output_get)) 40)
    (`TextRenderComponent.SetWorldSize` _messagetext 7.5)
    (else
      (`TextRenderComponent.SetWorldSize` _messagetext 10.0)))
  (`PaperZDAnimInstance.JumpToNode` (`PaperZDAnimationComponent.AnimInstance` (`self.AnimationComponent`)) "Airborne" "Locomotion"))

(fn `UserConstructionScript`)