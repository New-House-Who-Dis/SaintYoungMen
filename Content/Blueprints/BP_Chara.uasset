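; BP_Chara is a controllable 2D sprite character in a 3D world that can be clicked to show an introduction.
; Tick yaws the actor toward the camera, and movement input snaps that facing to a world axis for camera-relative directions.
; Horizontal input sets the sprite's X scale for facing, and jumping sends the animation state machine to Airborne.
; The first click opens a WB_Dialogue with the Introduction text, and later clicks remove it.
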(event `EnhancedInput|/Game/Characters/Input/Actions/IA_Jump`
  (params (ActionValue :type Boolean) (ElapsedSeconds :type "Float (double-precision)") (TriggeredSeconds :type "Float (double-precision)") (InputAction :type "InputAction Object Reference" :default "/Game/Characters/Input/Actions/IA_Jump.IA_Jump"))
  (:`Triggered`
    (`self.Jump`)))

(event `self.ReceiveBeginPlay`
  (bind _asplayer_controller (cast `PlayerController` (`self.GetController`)))
  (bind _returnvalue (pcsubsystem `EnhancedInputLocalPlayerSubsystem` _asplayer_controller))
  (`/Engine/EditorBlueprintResources/StandardMacros.IsValid` _returnvalue
    (:`Is Valid`
      (`EnhancedInputSubsystemInterface.AddMappingContext` _returnvalue "/Game/Characters/Input/IMC_Default.IMC_Default" 0 (struct)))))

(event `self.OnJumped`
  (`PaperZDAnimInstance.JumpToNode` (`PaperZDAnimationComponent.AnimInstance` (`self.AnimationComponent`)) "Airborne" "Locomotion"))

(event `EnhancedInput|/Game/Characters/Input/Actions/IA_Move`
  (params (ActionValue :type "Vector2D Structure") (ElapsedSeconds :type "Float (double-precision)") (TriggeredSeconds :type "Float (double-precision)") (InputAction :type "InputAction Object Reference" :default "/Game/Characters/Input/Actions/IA_Move.IA_Move"))
  (bind (_returnvalue_x _returnvalue_y) (`KismetMathLibrary.BreakVector` (`self.GetActorForwardVector`)))
  (:`Triggered`
    (if (> (`KismetMathLibrary.Abs` _returnvalue_x) (`KismetMathLibrary.Abs` _returnvalue_y))
      (if (> _returnvalue_x 0.0)
        (`self.AddMovementInput` (-1.0 0.0 0.0) ActionValue_Y)
        (`self.AddMovementInput` (0.0 -1.0 0.0) ActionValue_X)
        (else
          (`self.AddMovementInput` (1.0 0.0 0.0) ActionValue_Y)
          (`self.AddMovementInput` (0.0 1.0 0.0) ActionValue_X)))
      (elif (> _returnvalue_y 0.0)
        (`self.AddMovementInput` (0.0 -1.0 0.0) ActionValue_Y)
        (`self.AddMovementInput` (1.0 0.0 0.0) ActionValue_X)
        (else
          (`self.AddMovementInput` (0.0 1.0 0.0) ActionValue_Y)
          (`self.AddMovementInput` (-1.0 0.0 0.0) ActionValue_X))))
    (if (!= ActionValue_X 0.0)
      (bind _output_get (set `self.Directionality` ActionValue_X))
      (bind _result (`/Engine/EditorBlueprintResources/StandardMacros.NegateFloat` _output_get)
        (:`  `
          (`SceneComponent.SetWorldScale3D` (`self.Sprite`) (`KismetMathLibrary.MakeVector` _result 1.0 1.0)))))))

(event `self.ReceiveTick`
  (params (DeltaSeconds :type "Float (single-precision)"))
  (bind (_returnvalue_roll _returnvalue_pitch _returnvalue_yaw) (`KismetMathLibrary.BreakRotator` (`PlayerCameraManager.GetCameraRotation` (`GameplayStatics.GetPlayerCameraManager` 0))))
  (`self.K2_SetActorRotation` (`KismetMathLibrary.MakeRotator` 0.0 0.0 (- _returnvalue_yaw 180.0))))

(event `self.ReceiveActorOnClicked`
  (params (ButtonPressed :type "Key Structure"))
  (if (`self.Introduced`)
    (`Widget.RemoveFromParent` (`self.IntroUI`) :!label _label)
    (else
      (`self.IntroUI`
        (:`then`
          (goto _label))
        (:`else`
          (bind _returnvalue (`|CreateWidget` "/Game/Blueprints/WB_Dialogue.WB_Dialogue_C" (`GameplayStatics.GetPlayerController` 0)))
          (bind _output_get (set `self.IntroUI` _returnvalue))
          (`UserWidget.AddToViewport` _output_get 0)
          (`TextBlock.SetText` (`/Game/Blueprints/WB_Dialogue.DialogueText` (`self.IntroUI`)) (`KismetTextLibrary.Conv_StringToText` (`self.Introduction`)))
          (set `self.Introduced` true))))))

(fn `UserConstructionScript`)