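; MapPieceBp is a self-chaining track segment for an infinite runner, with randomly chosen meshes for two houses and an obstacle.
; The construction script picks those meshes from type arrays.
; When BP_Chara_Runner overlaps the Box, the piece raises its clamped speed, spawns the next piece at ArrowEnd, adds score and updates ScoreText.
; The piece destroys itself after a delay, clearing track behind the runner.
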(event `self.Box.OnComponentBeginOverlap`
  (params (OverlappedComponent :type "PrimitiveComponent Object Reference") (OtherActor :type "Actor Object Reference") (OtherComp :type "PrimitiveComponent Object Reference") (OtherBodyIndex :type Integer) (bFromSweep :type Boolean) (SweepResult :type "HitResult Structure (by ref)"))
  (bind _asbp_chara_runner (cast `/Game/Blueprints/BP_Chara_Runner` OtherActor))
  (set `/Game/Blueprints/BP_Chara_Runner.Speed` (`KismetMathLibrary.FClamp` (+ (`/Game/Blueprints/BP_Chara_Runner.Speed` _asbp_chara_runner) 0.07) 0.0 2.5) _asbp_chara_runner)
  (`|SpawnActorFromClass` "MapPieceBp_C" (`SceneComponent.K2_GetComponentToWorld` (`self.ArrowEnd`)) "Undefined" "MultiplyWithRoot" null null)
  (bind _returnvalue (+ (`/Game/Blueprints/BP_Chara_Runner.Score` _asbp_chara_runner) 10))
  (set `/Game/Blueprints/BP_Chara_Runner.Score` _returnvalue _asbp_chara_runner)
  (`TextRenderComponent.K2_SetText` (`self.ScoreText`) (`KismetTextLibrary.Conv_IntToText` _returnvalue false true 2))
  (`KismetSystemLibrary.Delay` 20.0)
  (`self.K2_DestroyActor`))

(event `self.ReceiveBeginPlay`)

(fn `UserConstructionScript`
  (bind _outitem (`KismetArrayLibrary.Array_Random` (`self.HouseTypes`)))
  (`StaticMeshComponent.SetStaticMesh` (`self.House1`) _outitem)
  (`StaticMeshComponent.SetStaticMesh` (`self.House2`) _outitem)
  (`StaticMeshComponent.SetStaticMesh` (`self.Obstacles`) (`KismetArrayLibrary.Array_Random` (`self.ObstacleTypes`))))